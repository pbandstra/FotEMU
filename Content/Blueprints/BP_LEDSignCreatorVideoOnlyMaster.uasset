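; Procedural LED sign actor whose construction script sweeps a profile spline along a path spline into mesh panels and reports its physical size.
; Each panel gets a dynamic material with LED, texture, motion and flipbook settings, offset in U by panel index.
; Optional text draws to a canvas render target, cycling entries by self-retriggering updates after per-entry delays, starting at BeginPlay or via an editor preview event.
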(event `self.ReceiveBeginPlay`
  (bind _textanddelay (`self.TextAndDelay`))
  (bind _canvas2d (`self.Canvas2D`))
  ;[1 1 1] Update Text Element (if using text-only mode) either OnBeginPlay or when required via editor exposed  custom event.
  (if (`self.bUseText?`) :!label _label
    (add `CanvasRenderTarget2D.OnCanvasRenderTargetUpdate` _canvas2d (delegate `CanvasUpdated`))
    (bind _output_get (set `self.TextArrayLength` (`BlueprintMapLibrary.Map_Length` (`self.TextAndDelay`))))
    (set `self.TextArrayCountIndex` 0)
    (set `self.TextArrayLastIndex` (- _output_get 1))
    (bind _keys (`BlueprintMapLibrary.Map_Keys` _textanddelay))
    (set `self.TextArrayText` _keys)
    (bind _values (`BlueprintMapLibrary.Map_Values` _textanddelay))
    (set `self.TextArrayDelay` _values)
    (`CanvasRenderTarget2D.UpdateResource` _canvas2d)))

(event `PreviewLiveTextInEditor`
  (goto _label))

(event `CanvasUpdated`
  (params (Canvas :type "Canvas Object Reference") (Width :type Integer) (Height :type Integer))
  ;[1 1 1] Update Text Element (if using text-only mode) either OnBeginPlay or when required via editor exposed  custom event.
  (`Canvas.K2_DrawText` Canvas (`self.Font`) (`|GetArrayItem` (`self.TextArrayText`) (`self.TextArrayCountIndex`)) (`self.TextPosition`) (1.0 1.0) (struct :`R` 1.0 :`G` 1.0 :`B` 1.0 :`A` 1.0) (`self.TextKerning`) (struct :`A` 1.0) (1.0 1.0) false false false (struct :`A` 1.0))
  (`KismetSystemLibrary.Delay` (`|GetArrayItem` (`self.TextArrayDelay`) (`self.TextArrayCountIndex`)))
  (if (>= (`self.TextArrayCountIndex`) (`self.TextArrayLastIndex`))
    (set `self.TextArrayCountIndex` 0)
    (else
      (`/Engine/EditorBlueprintResources/StandardMacros.IncrementInt` (`self.TextArrayCountIndex`)
        (:`  `
          _))))
  (if (>= (`self.TextArrayLength`) 2)
    (`CanvasRenderTarget2D.UpdateResource` (`self.Canvas2D`))))

(fn `CalculatePhysicalDimensions`
  (params (AlongSpline :type "SplineComponent Object Reference") (Spline :type "SplineComponent Object Reference"))
  (returns (MetricDimensions :type Name))
  (bind _returnvalue (`SplineComponent.GetSplineLength` Spline))
  (bind _returnvalue_2 (`SplineComponent.GetSplineLength` AlongSpline))
  (bind _returnvalue_3 (<= _returnvalue 100.0))
  (bind _returnvalue_4 (<= _returnvalue_2 100.0))
  (return (`KismetStringLibrary.Conv_StringToName` (`KismetStringLibrary.Concat_StrStr` "Width: " (`KismetTextLibrary.Conv_TextToString` (`KismetTextLibrary.Conv_DoubleToText` (`KismetMathLibrary.SelectFloat` _returnvalue_2 (/ _returnvalue_2 100.0) _returnvalue_4) "HalfToEven" false true 1 324 0 2)) (`KismetMathLibrary.SelectString` "cm" "m" _returnvalue_4) " x " "Height: " (`KismetTextLibrary.Conv_TextToString` (`KismetTextLibrary.Conv_DoubleToText` (`KismetMathLibrary.SelectFloat` _returnvalue (/ _returnvalue 100.0) _returnvalue_3) "HalfToEven" false true 1 324 0 2)) (`KismetMathLibrary.SelectString` "cm" "m" _returnvalue_3)))))

(fn `GenerateAlongSpline`
  (params (ProcMeshComponent :type "ProceduralMeshComponent Object Reference") (Spline :type "SplineComponent Object Reference") (AlongSpline :type "SplineComponent Object Reference") (Iterations :type Integer))
  (bind _array (`|MakeArray` (0.0 0.0) (0.0 1.0) (1.0 0.0) (1.0 1.0) :!type "Vector2D Structure"))
  (bind _panelwidth (`self.PanelWidth`))
  (bind _sides (`self.Sides`))
  (bind (_x _y) (`KismetMathLibrary.BreakVector2D` (`self.TextureAFlipbookColsRows`)))
  (bind (_x_2 _y_2) (`KismetMathLibrary.BreakVector2D` (`self.TextureBFlipbookColsRows`)))
  (bind (_x_3 _y_3) (`KismetMathLibrary.BreakVector2D` (`self.TexturesUVScale`)))
  (bind (_x_4 _y_4) (`KismetMathLibrary.BreakVector2D` (`self.PannerSpeed`)))
  (bind (_x_5 _y_5) (`KismetMathLibrary.BreakVector2D` (* (`self.LEDPixels`) (`self.LEDPixelsDPI`))))
  (for _index (range 1 (+ Iterations 1))
    (for _index_2 (range _sides)
      (bind _triangles (`KismetProceduralMeshLibrary.CreateGridMeshTriangles` 2 2))
      (bind _loc (`self.LocationAndRotationAlongSpline` Spline _sides _index_2))
      (bind (_loc_2 _rot) (`self.LocationAndRotationAlongSpline` AlongSpline Iterations (- _index 1)))
      (bind _loc_3 (`self.LocationAndRotationAlongSpline` Spline _sides (+ _index_2 1)))
      (bind (_loc_4 _rot_2) (`self.LocationAndRotationAlongSpline` AlongSpline Iterations _index))
      (bind _tri (`self.MapToTri` (+ (`KismetMathLibrary.GreaterGreater_VectorRotator` _loc _rot) _loc_2) (+ (`KismetMathLibrary.GreaterGreater_VectorRotator` _loc_3 _rot) _loc_2) (+ (`KismetMathLibrary.GreaterGreater_VectorRotator` _loc _rot_2) _loc_4) (+ (`KismetMathLibrary.GreaterGreater_VectorRotator` _loc_3 _rot_2) _loc_4)))
      (bind (_normals _tangents) (`KismetProceduralMeshLibrary.CalculateTangentsForMesh` _tri _triangles _array))
      ;[1 1 1] Create Mesh Section
      (`ProceduralMeshComponent.CreateMeshSection_LinearColor` :`self` ProcMeshComponent :`SectionIndex` _index :`Vertices` _tri :`Triangles` _triangles :`Normals` _normals :`UV0` _array :`VertexColors` (`self.VertexColors`) :`Tangents` _tangents)
      ;[1 1 1] Set Material Params
      (bind _returnvalue (`KismetMaterialLibrary.CreateDynamicMaterialInstance` (`self.Material`)))
      (switch `/Game/LED_Creator/Blueprints/ENUM_TextureRotation` (`self.TextureRotation`)
        (:`NewEnumerator0`
          (`MaterialInstanceDynamic.SetScalarParameterValue` _returnvalue "Rotation" 0.5))
        (:`NewEnumerator1`
          (`MaterialInstanceDynamic.SetScalarParameterValue` _returnvalue "Rotation" 0.25))
        (:`NewEnumerator2`
          (`MaterialInstanceDynamic.SetScalarParameterValue` _returnvalue "Rotation" -0.25))
        (:`NewEnumerator3`
          (`MaterialInstanceDynamic.SetScalarParameterValue` _returnvalue "Rotation" 0.0)))
      (`MaterialInstanceDynamic.SetScalarParameterValue` _returnvalue "Width" _panelwidth)
      (`MaterialInstanceDynamic.SetScalarParameterValue` _returnvalue "Uoffset" (* _panelwidth (`KismetMathLibrary.Conv_IntToDouble` (`self.IndexCounter`))))
      (`MaterialInstanceDynamic.SetScalarParameterValue` _returnvalue "LEDPixelResolutionX" _x_5)
      (`MaterialInstanceDynamic.SetScalarParameterValue` _returnvalue "LEDPixelResolutionY" _y_5)
      (`MaterialInstanceDynamic.SetScalarParameterValue` _returnvalue "TextureUScale" _x_3)
      (`MaterialInstanceDynamic.SetScalarParameterValue` _returnvalue "TextureVScale" _y_3)
      (`MaterialInstanceDynamic.SetScalarParameterValue` _returnvalue "PanSpeedX" _x_4)
      (`MaterialInstanceDynamic.SetScalarParameterValue` _returnvalue "PanSpeedY" _y_4)
      (switch `/Game/LED_Creator/Blueprints/ENUM_LEDShape` (`self.LED Shape`)
        (:`NewEnumerator0`
          (`MaterialInstanceDynamic.SetScalarParameterValue` _returnvalue "LedShape" 0.5))
        (:`NewEnumerator1`
          (`MaterialInstanceDynamic.SetScalarParameterValue` _returnvalue "LedShape" 1.0))
        (:`NewEnumerator2`
          (`MaterialInstanceDynamic.SetScalarParameterValue` _returnvalue "LedShape" 0.0)))
      (if (`self.bFlicker?`)
        (`MaterialInstanceDynamic.SetScalarParameterValue` _returnvalue "bFlicker" 1.0)
        (else
          (`MaterialInstanceDynamic.SetScalarParameterValue` _returnvalue "bFlicker" 0.0)))
      (`MaterialInstanceDynamic.SetVectorParameterValue` _returnvalue "TextureATint" (`self.TextureATint`))
      (`MaterialInstanceDynamic.SetVectorParameterValue` _returnvalue "TextureBTint" (`self.TextureBTint`))
      (switch `/Game/LED_Creator/Blueprints/ENUM_Motion` (`self.Motion`)
        (:`NewEnumerator0`
          (`MaterialInstanceDynamic.SetScalarParameterValue` _returnvalue "Motion" 0.0))
        (:`NewEnumerator1`
          (`MaterialInstanceDynamic.SetScalarParameterValue` _returnvalue "Motion" 0.5))
        (:`NewEnumerator2`
          (`MaterialInstanceDynamic.SetScalarParameterValue` _returnvalue "Motion" 1.0)))
      (`MaterialInstanceDynamic.SetScalarParameterValue` _returnvalue "EmissiveBoost" (`self.EmissiveBoost`))
      (`MaterialInstanceDynamic.SetScalarParameterValue` _returnvalue "TextureDPI" (`self.TexturesDPI`))
      (`MaterialInstanceDynamic.SetTextureParameterValue` _returnvalue "TextureA" (`self.TextureA`))
      (`MaterialInstanceDynamic.SetTextureParameterValue` _returnvalue "TextureB" (`self.TextureB`))
      ;;[1 1 1] Add Text
      (if (`self.bUseText?`)
        (`MaterialInstanceDynamic.SetTextureParameterValue` _returnvalue "TextTexture" (`self.Canvas2D`))
        (else
          (`MaterialInstanceDynamic.SetTextureParameterValue` _returnvalue "TextTexture" (`self.TextTexture_empty`))))
      (`MaterialInstanceDynamic.SetVectorParameterValue` _returnvalue "FontColor" (`self.FontColor`))
      (`MaterialInstanceDynamic.SetScalarParameterValue` _returnvalue "BumperSpeed" (`self.BumperSpeed`))
      (if (`self.bTextureAUseFlipbook?`)
        (`MaterialInstanceDynamic.SetScalarParameterValue` _returnvalue "TextureAUseFlipbook" 1.0)
        (`MaterialInstanceDynamic.SetScalarParameterValue` _returnvalue "TextureAFlipbookSpeed" (`self.TextureAFlipbookSpeed`))
        (`MaterialInstanceDynamic.SetScalarParameterValue` _returnvalue "TextureAFlipbookRows" _y)
        (`MaterialInstanceDynamic.SetScalarParameterValue` _returnvalue "TextureAFlipbookCols" _x)
        (else
          (`MaterialInstanceDynamic.SetScalarParameterValue` _returnvalue "TextureAUseFlipbook" 0.0)))
      (if (`self.bTextureBUseFlipbook?`)
        (`MaterialInstanceDynamic.SetScalarParameterValue` _returnvalue "TextureBUseFlipbook" 1.0)
        (`MaterialInstanceDynamic.SetScalarParameterValue` _returnvalue "TextureBFlipbookSpeed" (`self.TextureBFlipbookSpeed`))
        (`MaterialInstanceDynamic.SetScalarParameterValue` _returnvalue "TextureBFlipbookRows" _x_2)
        (`MaterialInstanceDynamic.SetScalarParameterValue` _returnvalue "TextureBFlipbookCols" _y_2)
        (else
          (`MaterialInstanceDynamic.SetScalarParameterValue` _returnvalue "TextureBUseFlipbook" 0.0)))
      ;[1 1 1] Each mesh section gets a new material index
      (`PrimitiveComponent.SetMaterial` ProcMeshComponent _index _returnvalue)
      ;[1 1 1] Avoids any funny business that may happen in CS loops
      (`/Engine/EditorBlueprintResources/StandardMacros.IncrementInt` (`self.IndexCounter`)))))

(fn `GenerateCustomMesh`
  (returns (ProcMeshComp :type "ProceduralMeshComponent Object Reference"))
  (bind _splineiterations (`self.SplineIterations`))
  ;[1 1 1] Create Procedural Mesh Component and Mesh Sections
  (bind _returnvalue (`AddComponent|NODE_AddProceduralMeshComponent-2`))
  (`self.GenerateAlongSpline` _returnvalue (`self.Spline`) (`self.AlongSpline`) _splineiterations)
  (set `self.TotalPolygonCount` (* _splineiterations 2))
  (return _returnvalue))

(fn `UpdateCanvas`
  (params (Canvas2D :type "CanvasRenderTarget2D Object Reference"))
  (`CanvasRenderTarget2D.UpdateResource` Canvas2D))

(fn `UserConstructionScript`
  ;[1 1 1] Reset Iteration Counter
  (set `self.IndexCounter` 0)
  ;[1 1 1] Calculate quad width
  (set `self.PanelWidth` (/ 1.0 (`KismetMathLibrary.Conv_IntToDouble` (`self.SplineIterations`))))
  (if (`self.bUseText?`)
    ;[1 1 1] Set up canvas
    (bind _returnvalue (`CanvasRenderTarget2D.CreateCanvasRenderTarget2D` "/Script/Engine.CanvasRenderTarget2D"))
    (set `self.Canvas2D` _returnvalue))
  ;[1 1 1] Generate Procedural Mesh
  (`self.GenerateCustomMesh`)
  ;[1 1 1] Calculate Physical Dimensions
  (bind _metricdimensions (`self.CalculatePhysicalDimensions` (`self.AlongSpline`) (`self.Spline`)))
  (set `self.PhysicalDimensions` _metricdimensions))